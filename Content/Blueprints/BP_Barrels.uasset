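; BP_Barrels is a barrel actor that tracks how long it keeps moving and feeds that time into a high score on GM_Barrels.
; Construction builds a dynamic material and swaps its texture set by the game mode's BarrelSelection.
; Tick adds to the game mode's shared timer while mesh speed exceeds a small threshold.
; The game mode's explode event resets that timer and destroys the barrel, optionally spawning an explosion effect.
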(event Custom|CE_Explode
  (if (Variables|/Game/Blueprints/GM_Barrels.GM_Barrels_C|GetBarrelExplode (Variables|Default|GetAs%20GM%20Barrels))
    (Effects|SpawnEmitteratLocation "/Game/FX/Particles/PS_ImpactExplosion3.PS_ImpactExplosion3" (Transformation|GetWorldLocation (Variables|Default|Getsm_Barrel))))
  (Variables|/Game/Blueprints/GM_Barrels.GM_Barrels_C|SetBarrelMovingTime (Variables|Default|GetAs%20GM%20Barrels) 0.0)
  (Actor|DestroyActor))

(event EventTick
  (params (DeltaSeconds :type Float%20%28single-precision%29))
  (bind _as_gm_barrels (Variables|Default|GetAs%20GM%20Barrels))
  (bind _as_gm_barrels_2 (Variables|Default|GetAs%20GM%20Barrels))
  (if (not (<= (Math|Vector|VectorLength (Transformation|GetComponentVelocity (Variables|Default|Getsm_Barrel))) 0.2))
    (bind _output_get (Variables|/Game/Blueprints/GM_Barrels.GM_Barrels_C|SetBarrelMovingTime _as_gm_barrels_2 (+ (Variables|/Game/Blueprints/GM_Barrels.GM_Barrels_C|GetBarrelMovingTime _as_gm_barrels_2) (Utilities|Time|GetWorldDeltaSeconds))))
    (if (> _output_get (Variables|/Game/Blueprints/GM_Barrels.GM_Barrels_C|GetHighScore _as_gm_barrels))
      (Variables|/Game/Blueprints/GM_Barrels.GM_Barrels_C|SetHighScore _as_gm_barrels _output_get))))

(event EventBeginPlay
  (bind _asgm_barrels (Utilities|Casting|CastToGM_Barrels (Game|GetGameMode)))
  (Variables|Default|SetAs%20GM%20Barrels _asgm_barrels)
  (EventDispatchers|BindEventtoEDExplode (Variables|Default|GetAs%20GM%20Barrels) (delegate Custom|CE_Explode)))

(fn ConstructionScript
  (bind _asgm_barrels (Utilities|Casting|CastToGM_Barrels (Game|GetGameMode)))
  (Variables|Default|SetAs%20GM%20Barrels _asgm_barrels)
  (bind _returnvalue (Rendering|Material|CreateDynamicMaterialInstance (Variables|Default|Getsm_Barrel) 0 "/Game/Textures/MM_Simple.MM_Simple" "None" :!class /Script/Engine.PrimitiveComponent))
  (Variables|Default|SetDynaMat _returnvalue)
  (switch int (Variables|/Game/Blueprints/GM_Barrels.GM_Barrels_C|GetBarrelSelection (Variables|Default|GetAs%20GM%20Barrels))
    (:1
      (Rendering|Material|SetTextureParameterValue (Variables|Default|GetDynaMat) "BaseColor" "/Game/Textures/Barrel01_BC.Barrel01_BC")
      (Rendering|Material|SetTextureParameterValue (Variables|Default|GetDynaMat) "Normal" "/Game/Textures/Barrel01_NORM.Barrel01_NORM")
      (Rendering|Material|SetTextureParameterValue (Variables|Default|GetDynaMat) "ARM" "/Game/Textures/Barrel01_ARM.Barrel01_ARM"))
    (:2
      (Rendering|Material|SetTextureParameterValue (Variables|Default|GetDynaMat) "BaseColor" "/Game/Textures/Barrel02_BC.Barrel02_BC")
      (Rendering|Material|SetTextureParameterValue (Variables|Default|GetDynaMat) "Normal" "/Game/Textures/Barrel02_NORM.Barrel02_NORM")
      (Rendering|Material|SetTextureParameterValue (Variables|Default|GetDynaMat) "ARM" "/Game/Textures/Barrel02_ARM.Barrel02_ARM"))
    (:3
      (Rendering|Material|SetTextureParameterValue (Variables|Default|GetDynaMat) "BaseColor" "/Game/Textures/Barrel03_BC.Barrel03_BC")
      (Rendering|Material|SetTextureParameterValue (Variables|Default|GetDynaMat) "Normal" "/Game/Textures/Barrel03_NORM.Barrel03_NORM")
      (Rendering|Material|SetTextureParameterValue (Variables|Default|GetDynaMat) "ARM" "/Game/Textures/Barrel03_ARM.Barrel03_ARM"))))